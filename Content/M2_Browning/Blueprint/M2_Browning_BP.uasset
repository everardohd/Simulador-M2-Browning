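; Mountable-style M2 Browning machine gun Blueprint that fires projectiles on the Fire input.
; Each shot spawns a projectile at the muzzle socket with slight random pitch and yaw spread, plus a firing sound and scaled-down emitter.
; Pressing Fire shoots, plays a montage and sets a timer by function name for a further shot, which release clears.
; Turn and LookUp inputs do nothing, as their clamped aim logic is disconnected.
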(event `InputAxis|LookUp`
  (params (AxisValue :type "Float (single-precision)")))

(event `InputAxis|Turn`
  (params (AxisValue :type "Float (single-precision)")))

(event `Spawn Projectile`
  (bind (_returnvalue_location _returnvalue_rotation _returnvalue_scale) (`KismetMathLibrary.BreakTransform` (`KismetMathLibrary.MakeTransform` (.location (`SceneComponent.GetSocketTransform` (`self.M2_Browning`) "M2_Fire_Socket" "RTS_World")) (`KismetMathLibrary.MakeRotator` 0.0 (+ (.pitch (.rotation (`SceneComponent.GetSocketTransform` (`self.M2_Browning`) "M2_Fire_Socket" "RTS_World"))) (`KismetMathLibrary.RandomFloatInRange` -1.0 1.0)) (+ (.yaw (.rotation (`SceneComponent.GetSocketTransform` (`self.M2_Browning`) "M2_Fire_Socket" "RTS_World"))) (`KismetMathLibrary.RandomFloatInRange` -1.0 1.0))))))
  (`|SpawnActorFromClass` "/Game/FirstPersonBP/Blueprints/FirstPersonProjectile.FirstPersonProjectile_C" (`KismetMathLibrary.MakeTransform` _returnvalue_location _returnvalue_rotation _returnvalue_scale) "Undefined" "OverrideRootScale" null null)
  (`GameplayStatics.PlaySoundAtLocation` "/Game/M2_Browning/Bullet/M2_Shoot.M2_Shoot" (`self.K2_GetActorLocation`)) ; Play firing sound
  (bind _returnvalue (`GameplayStatics.SpawnEmitterAtLocation` "/Game/M2_Browning/Particles/M2_Explosion.M2_Explosion" _returnvalue_location _returnvalue_rotation))
  (`SceneComponent.SetWorldScale3D` _returnvalue (0.3 0.3 0.3)))

(event `InputAction|Fire`
  (params (Key :type "Key Structure"))
  (:`Pressed`
    (`self.Spawn Projectile`)
    (set `self.IsFiring?` true)
    (`AnimInstance.Montage_Play` (`SkeletalMeshComponent.GetAnimInstance` (`self.M2_Browning`)) null 1.0 "MontageLength" 0.0)
    (`KismetSystemLibrary.K2_SetTimer` null "Spawn Projectile" 20.0))
  (:`Released`
    (set `self.IsFiring?` false)
    (`KismetSystemLibrary.K2_ClearTimer` null "Spawn Projectile")))

(fn `UserConstructionScript`)